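; Player controller that turns input into movement, look, jump and weapon fire for the first local player.
; Move axes push pawn 0 along the controller's own forward and right vectors rather than the pawn's.
; Look axes scale yaw and pitch by frame delta time and a shared TurnRate.
; Jump calls the character directly, while Fire casts to BP_Player, calls FireWeapon and increments ShootCount.
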(event Input|ActionEvents|InputActionJump
  (params (Key :type Key%20Structure :default "None"))
  (:Pressed
    (Character|Jump (Game|GetPlayerCharacter 0))))

(event Input|ActionEvents|InputActionFire
  (params (Key :type Key%20Structure :default "None"))
  (:Pressed
    (bind _asbp_player (Utilities|Casting|CastToBP_Player (Game|GetPlayerCharacter 0)))
    (Default|FireWeapon _asbp_player)
    (Math|Integer|IncrementInt (Variables|Default|GetShootCount))))

(event Input|AxisEvents|InputAxisMoveForward
  (params (AxisValue :type Float%20%28single-precision%29))
  (Pawn|Input|AddMovementInput (Game|Player|GetPlayerPawn 0) (Transformation|GetActorForwardVector) AxisValue false))

(event Input|AxisEvents|InputAxisMoveRight
  (params (AxisValue :type Float%20%28single-precision%29))
  (Pawn|Input|AddMovementInput (Game|Player|GetPlayerPawn 0) (Transformation|GetActorRightVector) AxisValue false))

(event Input|AxisEvents|InputAxisTurn
  (params (AxisValue :type Float%20%28single-precision%29))
  (Class|PlayerController|AddYawInput (* AxisValue (Utilities|Time|GetWorldDeltaSeconds) (Variables|Default|GetTurnRate))))

(event Input|AxisEvents|InputAxisLookUp
  (params (AxisValue :type Float%20%28single-precision%29))
  (Class|PlayerController|AddPitchInput (* AxisValue (Utilities|Time|GetWorldDeltaSeconds) (Variables|Default|GetTurnRate))))

(fn ConstructionScript)